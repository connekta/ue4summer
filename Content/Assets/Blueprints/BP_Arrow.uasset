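; Arrow actor that players pick up into the right-hand socket, launch as a projectile, and can kill other players with.
; Occupied and attacking flags gate pickup, and launching detaches it and enables projectile movement with reduced gravity.
; While flying, overlaps call KillMe on players, and a delayed downward trace from Tick detects nearby ground.
; A successful kill or ground proximity stops it and drops it to the traced surface.
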(event `self.ReceiveActorBeginOverlap`
  (params (OtherActor :type "Actor Object Reference"))
  (if (`self.is_attacking`)
    (bind _asbp_player (cast `/Game/Assets/Blueprints/BP_Player` OtherActor))
    (bind _result (`/Game/Assets/Blueprints/BP_Player.KillMe` _asbp_player))
    (if _result
      (`self.StopProjectile`))))

(event `self.ReceiveTick`
  (params (DeltaSeconds :type "Float (single-precision)"))
  (bind _returnvalue (`self.K2_GetActorLocation`))
  (if (`self.is_attacking`)
    (`KismetSystemLibrary.Delay` 0.2)
    (bind _outhit (`KismetSystemLibrary.LineTraceSingle` _returnvalue (- _returnvalue (0.0 0.0 100000.0)) "TraceTypeQuery1"))
    (bind (_bblockinghit _binitialoverlap _time _distance _location _impactpoint _normal _impactnormal _physmat _hitactor) (`GameplayStatics.BreakHitResult` _outhit))
    (cast `/Game/Assets/Blueprints/BP_Player` _hitactor
      (:`CastFailed`
        (if (< _distance 10.0)
          (`self.StopProjectile`))))))

(fn `DisplayDebugTrajectory`
  (params (Velocity :type "Vector Structure"))
  (`GameplayStatics.Blueprint_PredictProjectilePath_ByTraceChannel` :`StartPos` (`self.K2_GetActorLocation`) :`LaunchVelocity` Velocity :`bTracePath` false :`DrawDebugType` "ForOneFrame" :`OverrideGravityZ` (`MovementComponent.GetGravityZ` (`self.ProjectileMovement`))))

(fn `IsReadyToBeTaken`
  (returns (Result :type Boolean))
  (return (not (or (`self.is_occupied`) (`self.is_attacking`)))))

(fn `SetupProjectile`
  (params (Direction :type "Vector Structure"))
  (bind _projectilemovement (`self.ProjectileMovement`))
  (`self.K2_DetachFromActor` "KeepWorld" "KeepWorld")
  (set `ProjectileMovementComponent.bSimulationEnabled` true _projectilemovement)
  (set `MovementComponent.Velocity` Direction _projectilemovement)
  (set `ProjectileMovementComponent.ProjectileGravityScale` 0.3 _projectilemovement)
  (set `self.is_attacking` true)
  (set `self.is_occupied` false))

(fn `StopProjectile`
  (bind _returnvalue (`self.K2_GetActorLocation`))
  (set `ProjectileMovementComponent.bSimulationEnabled` false (`self.ProjectileMovement`))
  (set `self.is_attacking` false)
  (bind _outhit (`KismetSystemLibrary.LineTraceSingle` _returnvalue (- _returnvalue (0.0 0.0 100000.0)) "TraceTypeQuery1"))
  (`self.K2_SetActorLocation` (`.Location` (`GameplayStatics.BreakHitResult` _outhit)) true true))

(fn `TakeMe`
  (params (Player :type "/Game/Assets/Blueprints/BP_Player Object Reference"))
  (set `self.is_occupied` true)
  (`PrimitiveComponent.SetCollisionEnabled` (`self.body`) "NoCollision")
  (`self.K2_AttachToActor` Player "RightHandSocket" "SnapToTarget" "SnapToTarget" "KeepRelative" false)
  (`self.K2_SetActorRelativeLocation` (0.0 0.0 0.0) false true)
  (`self.K2_SetActorRelativeRotation` (struct) false true)
  (return))

(fn `UserConstructionScript`)