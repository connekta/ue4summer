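; BP_Camera is a shared camera for local multiplayer that zooms according to how spread out the actors in GM_LocalMP's SpawnedActors are.
; On BeginPlay and every Tick, it builds a min/max box from those actors' bounds origins.
; The box's diagonal, clamped, sets the spring arm length, and up to four player controllers get this camera as view target.
; The graph changes only arm length, never the camera actor's position.
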(event `self.ReceiveBeginPlay`
  (`|ExecutionSequence` :!label _label
    (:`then_0`
      (set `self.bb_min` (0.0 0.0 0.0))
      (set `self.bb_max` (0.0 0.0 0.0)))
    (:`then_1`
      (bind _asgm_local_mp (cast `/Game/Assets/Blueprints/GM_LocalMP` (`GameplayStatics.GetGameMode`)))
      (for (_array_element _array_index) (`/Game/Assets/Blueprints/GM_LocalMP.SpawnedActors` _asgm_local_mp)
        (if (== _array_index 0)
          (bind _origin (`self.GetActorBounds` _array_element true))
          (set `self.bb_min` _origin)
          (set `self.bb_max` _origin)
          (else
            (set `self.bb_min` (`KismetMathLibrary.Vector_ComponentMin` _origin (`self.bb_min`)))
            (set `self.bb_max` (`KismetMathLibrary.Vector_ComponentMax` _origin (`self.bb_max`)))))))
    (:`then_2`
      (for _index (range 4)
        (bind _returnvalue (`GameplayStatics.GetPlayerController` _index))
        (`/Engine/EditorBlueprintResources/StandardMacros.IsValid` _returnvalue
          (:`Is Valid`
            (set `SpringArmComponent.TargetArmLength` (`KismetMathLibrary.FClamp` (`KismetMathLibrary.Vector_Distance` (`self.bb_min`) (`self.bb_max`)) 300.0 1000.0) (`self.SpringArm`))
            (`PlayerController.SetViewTargetWithBlend` _returnvalue self 0.0 "VTBlend_Linear" 0.0 false)))))))

(event `self.ReceiveTick`
  (params (DeltaSeconds :type "Float (single-precision)"))
  (goto _label))

(fn `UserConstructionScript`)