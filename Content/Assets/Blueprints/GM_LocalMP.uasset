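; Game mode for local multiplayer that creates a player for each PlayerStart, using its tag as controller and player ID.
; On BeginPlay it spawns and possesses BP_Player pawns, points up to four controllers at one shared camera, and restores shirt colors from the GameInstance.
; It shows a game-over widget once all players die, and saves colors before loading another level.
; A debug function hands controller 0 a chosen pawn.
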(event `self.ReceiveBeginPlay`
  ;[1 1 1] Spawn players and fill spawned actors array to use later in a code
  (`self.GetAllPlayerStarts`)
  (`self.SpawnPlayers`)
  (`|ExecutionSequence`
    (:`then_0`
      (for _index (range 4)
        (bind _returnvalue (`GameplayStatics.GetPlayerController` _index))
        (`/Engine/EditorBlueprintResources/StandardMacros.IsValid` _returnvalue
          (:`Is Valid`
            (`PlayerController.SetViewTargetWithBlend` _returnvalue (`self.MainCameraRef`) 0.0 "VTBlend_Linear" 0.0 false)))))
    (:`then_1`
      (bind _asbp_game_instance (cast `/Game/Assets/Blueprints/BP_GameInstance` (`GameplayStatics.GetGameInstance`)))
      (for (_array_element _array_index) (`self.SpawnedActors`)
        (set `/Game/Assets/Blueprints/BP_Player.CurrentShirtColor` (`|GetArrayItem` (`/Game/Assets/Blueprints/BP_GameInstance.PlayerColors` _asbp_game_instance) _array_index) _array_element)))))

(event `PlayerDead`
  ;[1 1 1] Check if all players dead -> Game Over!
  (set `self.number_of_dead_players` 0)
  (for _array_element (`self.SpawnedActors`)
    (if (`/Game/Assets/Blueprints/BP_Player.is_dead` _array_element)
      (`/Engine/EditorBlueprintResources/StandardMacros.IncrementInt` (`self.number_of_dead_players`))
      (else
        (break))))
  (if (== (`self.number_of_dead_players`) (`KismetArrayLibrary.Array_Length` (`self.SpawnedActors`)))
    (bind _returnvalue (`|CreateWidget` "/Game/Levels/GameOverWidget.GameOverWidget_C"))
    (`UserWidget.AddToViewport` _returnvalue 0)
    (bind _returnvalue_2 (`GameplayStatics.GetCurrentLevelName` true))
    (set `/Game/Levels/GameOverWidget.NextLevel` (`KismetStringLibrary.Conv_StringToName` _returnvalue_2) _returnvalue)
    (`WidgetBlueprintLibrary.SetInputMode_UIOnlyEx` (`GameplayStatics.GetPlayerController` 0) (`/Game/Levels/GameOverWidget.Button_Menu` _returnvalue))))

(fn `DebugTakeControl`
  (params (MainPlayerIndex :type Integer))
  (bind _spawnedactors (`self.SpawnedActors`))
  (`|ExecutionSequence`
    (:`then_0`
      ;[1 1 1] detach all player controls
      (for _index (range 4)
        (bind _returnvalue (`GameplayStatics.GetPlayerController` _index))
        (`/Engine/EditorBlueprintResources/StandardMacros.IsValid` _returnvalue
          (:`Is Valid`
            (`Controller.UnPossess` _returnvalue)))))
    (:`then_1`
      ;[1 1 1] rearrange indices
      (for (_array_element _array_index) _spawnedactors
        (bind _asbp_player (cast `/Game/Assets/Blueprints/BP_Player` _array_element))
        (if (== _array_index 0)
          (set `/Game/Assets/Blueprints/BP_Player.player_id` MainPlayerIndex _asbp_player)
          (elif (== MainPlayerIndex _array_index)
            (set `/Game/Assets/Blueprints/BP_Player.player_id` 0 _asbp_player)))))
    (:`then_2`
      (`Controller.Possess` (`GameplayStatics.GetPlayerController` 0) (`|GetArrayItem` _spawnedactors MainPlayerIndex)))))

(fn `GetAllPlayerStarts`
  (bind _outactors (`GameplayStatics.GetAllActorsOfClass` "/Script/Engine.PlayerStart"))
  (set `self.PlayerStartsArray` _outactors))

(fn `LoadNextLevel`
  (params (LevelName :type Name))
  (bind _asbp_game_instance (cast `/Game/Assets/Blueprints/BP_GameInstance` (`GameplayStatics.GetGameInstance`)))
  (for (_array_element _array_index) (`self.SpawnedActors`)
    (`KismetArrayLibrary.Array_Set` (`/Game/Assets/Blueprints/BP_GameInstance.PlayerColors` _asbp_game_instance) _array_index (`/Game/Assets/Blueprints/BP_Player.CurrentShirtColor` _array_element) true))
  (`GameplayStatics.OpenLevel` LevelName false)
  (`WidgetBlueprintLibrary.SetInputMode_GameOnly` (`GameplayStatics.GetPlayerController` 0))
  (`WidgetBlueprintLibrary.SetInputMode_GameOnly` (`GameplayStatics.GetPlayerController` 1))
  (`WidgetBlueprintLibrary.SetInputMode_GameOnly` (`GameplayStatics.GetPlayerController` 2))
  (`WidgetBlueprintLibrary.SetInputMode_GameOnly` (`GameplayStatics.GetPlayerController` 3)))

(fn `SpawnPlayers`
  (locals (PlayerIndex :type Integer))
  (`|ExecutionSequence`
    (:`then_0`
      (for _array_element (`self.PlayerStartsArray`)
        (bind _returnvalue (`KismetStringLibrary.Conv_StringToInt` (`KismetStringLibrary.Conv_NameToString` (`PlayerStart.PlayerStartTag` _array_element))))
        (`GameplayStatics.CreatePlayer` _returnvalue)
        (bind _returnvalue_2 (`|SpawnActorFromClass` "/Game/Assets/Blueprints/BP_Player.BP_Player_C" (`self.GetTransform` _array_element) "AlwaysSpawn" "OverrideRootScale" null null))
        (set `/Game/Assets/Blueprints/BP_Player.player_id` _returnvalue _returnvalue_2)
        (bind _returnvalue_3 (`GameplayStatics.GetPlayerController` _returnvalue))
        (`/Engine/EditorBlueprintResources/StandardMacros.IsValid` _returnvalue_3
          (:`Is Valid`
            (`Controller.Possess` _returnvalue_3 _returnvalue_2))
          (:`Is Not Valid`
            ;[1 1 1] For some reason one of 4 players are not spawning
            (`KismetSystemLibrary.PrintText` (`KismetTextLibrary.Conv_IntToText` _returnvalue))))
        (`KismetArrayLibrary.Array_AddUnique` (`self.SpawnedActors`) _returnvalue_2)))))

(fn `UserConstructionScript`)