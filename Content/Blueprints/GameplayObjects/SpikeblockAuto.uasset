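; SpikeblockAuto is a hazard block whose spikes move on their own from BeginPlay and kill the player on contact.
; A Timeline lerps the Spikes component from its starting relative location to a Z of SetHeight, also stretching its Z scale when that height exceeds a threshold.
; Overlapping KillTrigger calls KillMe on BP_Player.
; The interaction events are empty, so interaction has no effect.
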(event `self.ReceiveBeginPlay`
  (bind _spikes (`self.spikes`))
  (bind _relativelocation (`SceneComponent.RelativeLocation` (`self.spikes`)))
  (set `self.StartPos` _relativelocation)
  (set `self.EndPos` (`KismetMathLibrary.MakeVector` (.x _relativelocation) (.y _relativelocation) (`self.SetHeight`)))
  (bind (_direction _newtrack_0) (`Timeline|Timeline_0`)
    (:`Update`
      (`|ExecutionSequence`
        (:`then_0`
          (`SceneComponent.K2_SetRelativeLocation` _spikes (`KismetMathLibrary.VLerp` (`self.StartPos`) (`self.EndPos`) _newtrack_0) false false))
        (:`then_1`
          (if (> (`self.SetHeight`) 150.0)
            (`SceneComponent.SetRelativeScale3D` _spikes (`KismetMathLibrary.VLerp` (1.0 1.0 1.0) (1.0 1.0 1.5) _newtrack_0))))))))

(event `/Game/Blueprints/InteractableObject.InteractedEvent`)

(event `/Game/Blueprints/InteractableObject.StopedInteractedEvent`)

(event `self.KillTrigger.OnComponentBeginOverlap`
  (params (OverlappedComponent :type "PrimitiveComponent Object Reference") (OtherActor :type "Actor Object Reference") (OtherComp :type "PrimitiveComponent Object Reference") (OtherBodyIndex :type Integer) (bFromSweep :type Boolean) (SweepResult :type "HitResult Structure (by ref)"))
  (bind _asbp_player (cast `/Game/Assets/Blueprints/BP_Player` OtherActor))
  (`/Game/Assets/Blueprints/BP_Player.KillMe` _asbp_player))

(fn `UserConstructionScript`)