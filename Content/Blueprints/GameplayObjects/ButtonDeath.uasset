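; ButtonDeath is a trigger that activates two linked objects when the player dies after entering its box.
; Overlap by BP_Player starts isPlayerDead, which re-arms itself on a looping timer to poll IsDead.
; On death, a DoOnce sends InteractedEventMessage to Object and Object2, then attempts to clear the timer by name.
; End overlap also tries to clear it, but compares against Player, whose assignment never runs.
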(event `self.ReceiveTick`
  (params (DeltaSeconds :type "Float (single-precision)")))

(event `isPlayerDead`
  (`KismetSystemLibrary.K2_SetTimerDelegate` (delegate `isPlayerDead`) 0.5 true)
  (if (`/Game/Assets/Blueprints/BP_Player.is_dead` (stale `self.TriggerBox.OnComponentBeginOverlap` _asbp_player))
    (`/Engine/EditorBlueprintResources/StandardMacros.DoOnce` false
      (:`Completed`
        (message `/Game/Blueprints/InteractableObject.InteractedEvent` (`self.Object`))
        (message `/Game/Blueprints/InteractableObject.InteractedEvent` (`self.Object2`))
        (`KismetSystemLibrary.K2_ClearTimer` null "isPlayerDead")))))

(event `self.TriggerBox.OnComponentBeginOverlap`
  (params (OverlappedComponent :type "PrimitiveComponent Object Reference") (OtherActor :type "Actor Object Reference") (OtherComp :type "PrimitiveComponent Object Reference") (OtherBodyIndex :type Integer) (bFromSweep :type Boolean) (SweepResult :type "HitResult Structure (by ref)"))
  (bind _asbp_player (cast `/Game/Assets/Blueprints/BP_Player` OtherActor))
  (`self.isPlayerDead`))

(event `self.TriggerBox.OnComponentEndOverlap`
  (params (OverlappedComponent :type "PrimitiveComponent Object Reference") (OtherActor :type "Actor Object Reference") (OtherComp :type "PrimitiveComponent Object Reference") (OtherBodyIndex :type Integer))
  (if (== OtherActor (`self.player`))
    (`KismetSystemLibrary.K2_ClearTimer` null "isPlayerDead")))

(fn `NewFunction_0`)

(fn `UserConstructionScript`)