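; Gate01 is a gate Blueprint that responds to InteractedEvent by moving its Billboard component vertically.
; The GateTranslate timeline sets the component's relative Z to its track value times Height, keeping X and Y.
; A Gate boolean chooses between playing and reversing the timeline, but it starts true and the play branch sets it true again, so the reverse branch is never reached.
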(event `self.ReceiveBeginPlay`
  (set `self.gate` true))

(event `/Game/Blueprints/InteractableObject.InteractedEvent`
  (if (`self.gate`)
    (set `self.gate` true)
    (bind (_direction _newtrack_0) (`Timeline|GateTranslate` :!label _label)
      (:`Update`
        (`SceneComponent.K2_SetRelativeLocation` (`self.Billboard`) (`KismetMathLibrary.MakeVector` (.x (`SceneComponent.RelativeLocation` (`self.Billboard`))) (.y (`SceneComponent.RelativeLocation` (`self.Billboard`))) (* _newtrack_0 (`self.Height`))) false false)))
    (else
      (set `self.gate` false)
      (goto _label :!via `Reverse`))))

(fn `UserConstructionScript`)