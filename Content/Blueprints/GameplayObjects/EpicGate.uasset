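; A gate that swings open while its counter of activated buttons exactly equals the required number, and swings back otherwise.
; Up and down counter events adjust the current amount, which starts at zero on play.
; Every tick compares it to the needed count and plays or reverses two timelines that drive the yaw of two billboard components acting as the gate halves.
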(event `/Game/Blueprints/InteractableObject.InteractedEvent`)

(event `UpCounter`
  (set `self.CurrentAmount` (+ (`self.CurrentAmount`) 1)))

(event `DownCounter`
  (set `self.CurrentAmount` (- (`self.CurrentAmount`) 1)))

(event `self.ReceiveTick`
  (params (DeltaSeconds :type "Float (single-precision)"))
  (bind _billboard (`self.Billboard`))
  (bind _billboard1 (`self.Billboard1`))
  (if (== (`self.CurrentAmount`) (`self.ButtonsNeeded`))
    (`|ExecutionSequence`
      (:`then_0`
        (bind (_direction _newtrack_0) (`Timeline|gate0` :!label _label)
          (:`Update`
            (`SceneComponent.K2_SetRelativeRotation` _billboard (`KismetMathLibrary.MakeRotator` (.roll (`SceneComponent.RelativeRotation` _billboard)) (.pitch (`SceneComponent.RelativeRotation` _billboard)) _newtrack_0) false false))))
      (:`then_1`
        (bind (_direction_2 _newtrack_0_2) (`Timeline|gate01` :!label _label_2)
          (:`Update`
            (`SceneComponent.K2_SetRelativeRotation` _billboard1 (`KismetMathLibrary.MakeRotator` (.roll (`SceneComponent.RelativeRotation` _billboard1)) (.pitch (`SceneComponent.RelativeRotation` _billboard1)) _newtrack_0_2) false false)))))
    (else
      (`|ExecutionSequence`
        (:`then_0`
          (goto _label :!via `Reverse`))
        (:`then_1`
          (goto _label_2 :!via `Reverse`))))))

(event `self.ReceiveBeginPlay`
  (set `self.CurrentAmount` 0))

(fn `UserConstructionScript`)