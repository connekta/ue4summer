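; Interactable elevator Blueprint that moves its Parent component from its starting location to the DestinationPosition marker.
; On interaction, the Rise_elevator timeline lerps the platform position and scales four rope meshes in Z, with target length mapped from the height difference.
; A Gate flag chooses play or reverse, but stays true as written, so the reverse branch never runs.
; The construction script's StartDown check does nothing.
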(event `self.ReceiveBeginPlay`
  (set `self.Gate` true)
  (set `self.EndPos` (`SceneComponent.RelativeLocation` (`self.DestinationPosition`)))
  (set `self.StartPos` (`SceneComponent.RelativeLocation` (`self.parent`)))
  (`self.SetRelativeScale3D` (`self.elevator_rope2`) (1.0 1.0 0.15))
  (`self.SetRelativeScale3D` (`self.elevator_rope3`) (1.0 1.0 0.15))
  (`self.SetRelativeScale3D` (`self.elevator_rope`) (1.0 1.0 0.15))
  (`self.SetRelativeScale3D` (`self.elevator_rope1`) (1.0 1.0 0.15)))

(event `/Game/Blueprints/InteractableObject.InteractedEvent`
  (bind (_endpos_x _endpos_y _endpos_z) (`KismetMathLibrary.BreakVector` (`self.EndPos`)))
  (bind (_startpos_x _startpos_y _startpos_z) (`KismetMathLibrary.BreakVector` (`self.StartPos`)))
  (bind (_relativescale3d_x _relativescale3d_y _relativescale3d_z) (`KismetMathLibrary.BreakVector` (`SceneComponent.RelativeScale3D` (`self.elevator_rope1`))))
  (set `self.RopeLength` (- _endpos_z _startpos_z))
  (set `self.RopeScale` _relativescale3d_z)
  (if (`self.Gate`)
    (set `self.Gate` true)
    (bind (_direction _newtrack_0) (`Timeline|rise_elevator` :!label _label)
      (:`Update`
        (`|ExecutionSequence`
          (:`then_0`
            (`self.K2_SetRelativeLocation` (`self.parent`) (`KismetMathLibrary.VLerp` (`self.StartPos`) (`self.EndPos`) _newtrack_0) false false))
          (:`then_1`
            (`self.SetRelativeScale3D` (`self.elevator_rope2`) (`KismetMathLibrary.MakeVector` 1.0 1.0 (`KismetMathLibrary.Lerp` (`self.RopeScale`) (`KismetMathLibrary.MapRangeUnclamped` (`self.RopeLength`) 0.0 -180.0 0.15 1.0) _newtrack_0)))
            (`self.SetRelativeScale3D` (`self.elevator_rope3`) (`KismetMathLibrary.MakeVector` 1.0 1.0 (`KismetMathLibrary.Lerp` (`self.RopeScale`) (`KismetMathLibrary.MapRangeUnclamped` (`self.RopeLength`) 0.0 -180.0 0.15 1.0) _newtrack_0)))
            (`self.SetRelativeScale3D` (`self.elevator_rope`) (`KismetMathLibrary.MakeVector` 1.0 1.0 (`KismetMathLibrary.Lerp` (`self.RopeScale`) (`KismetMathLibrary.MapRangeUnclamped` (`self.RopeLength`) 0.0 -180.0 0.15 1.0) _newtrack_0)))
            (`self.SetRelativeScale3D` (`self.elevator_rope1`) (`KismetMathLibrary.MakeVector` 1.0 1.0 (`KismetMathLibrary.Lerp` (`self.RopeScale`) (`KismetMathLibrary.MapRangeUnclamped` (`self.RopeLength`) 0.0 -180.0 0.15 1.0) _newtrack_0)))))))
    (else
      (set `self.Gate` false)
      (goto _label :!via `Reverse`))))

(fn `UserConstructionScript`
  (if (`self.StartDown?`)
    _))