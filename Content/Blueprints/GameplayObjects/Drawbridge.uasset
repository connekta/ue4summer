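; Drawbridge actor that swings its Bridge component between its starting rotation and a fixed target when interacted with.
; The construction script sets a down or default starting pose from StartBridgeDown and caches it as StartPos.
; Each InteractedEvent flips the Gate flag to alternately play or reverse the RotActor timeline, whose RotBridge track drives the rotation lerp.
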(event `self.ReceiveBeginPlay`
  (set `self.Gate` true))

(event `/Game/Blueprints/InteractableObject.InteractedEvent`
  (if (`self.Gate`)
    (set `self.Gate` false)
    (bind (_direction _rotbridge) (`Timeline|RotActor` :!label _label)
      (:`Update`
        (`SceneComponent.K2_SetRelativeRotation` (`self.Bridge`) (`KismetMathLibrary.RLerp` (`self.StartPos`) (struct :`Roll` 90.0) _rotbridge) false false)))
    (else
      (set `self.Gate` true)
      (goto _label :!via `Reverse`))))

(fn `UserConstructionScript`
  (bind _bridge (`self.Bridge`))
  (if (`self.StartBridgeDown`)
    (`SceneComponent.K2_SetRelativeRotation` _bridge (struct :`Roll` 175.0) false false)
    (else
      (`SceneComponent.K2_SetRelativeRotation` _bridge (struct) false false)))
  (set `self.StartPos` (`SceneComponent.RelativeRotation` _bridge)))