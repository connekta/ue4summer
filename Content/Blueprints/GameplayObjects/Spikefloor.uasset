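; Spike floor trap that kills any BP_Player overlapping its KillTrigger by calling KillMe.
; The Cube starts without collision, and the first player kill makes it solid and visible and sets IsTriggered.
; A Timeline then lerps Spikebase1 and Cube upward once, with DoOnce never reset, while later overlaps still kill and unhide the player.
; An input-disabling branch is left unconnected.
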(event `self.KillTrigger.OnComponentBeginOverlap`
  (params (OverlappedComponent :type "PrimitiveComponent Object Reference") (OtherActor :type "Actor Object Reference") (OtherComp :type "PrimitiveComponent Object Reference") (OtherBodyIndex :type Integer) (bFromSweep :type Boolean) (SweepResult :type "HitResult Structure (by ref)"))
  (bind _cube (`self.Cube`))
  (bind _asbp_player (cast `/Game/Assets/Blueprints/BP_Player` OtherActor))
  (`/Game/Assets/Blueprints/BP_Player.KillMe` _asbp_player)
  (`self.SetActorHiddenInGame` OtherActor false)
  (`/Engine/EditorBlueprintResources/StandardMacros.DoOnce` false
    (:`Completed`
      (`PrimitiveComponent.SetCollisionEnabled` _cube "QueryAndPhysics")
      (set `self.is_triggered` true)
      (`KismetSystemLibrary.PrintString` "Hello")
      (`SceneComponent.SetVisibility` _cube true false)
      (bind (_direction _newtrack_0) (`Timeline|Timeline_0` :!via `PlayFromStart`)
        (:`Update`
          (`SceneComponent.K2_SetRelativeLocation` (`self.spikebase1`) (`KismetMathLibrary.MakeVector` 0.0 0.0 (`KismetMathLibrary.Lerp` -65.0 10.0 _newtrack_0)) false false)
          (`SceneComponent.K2_SetRelativeLocation` (`self.Cube`) (`KismetMathLibrary.MakeVector` 0.0 0.0 (`KismetMathLibrary.Lerp` -65.0 10.0 _newtrack_0)) false false))))))

(event `self.ReceiveBeginPlay`
  (`PrimitiveComponent.SetCollisionEnabled` (`self.Cube`) "NoCollision"))

(fn `UserConstructionScript`)