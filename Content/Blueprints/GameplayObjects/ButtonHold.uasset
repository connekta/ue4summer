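; Pressure button that stays active while something overlaps its trigger box.
; Overlap begin and end send Interacted and StopedInteracted event messages to two referenced objects, Object and Object2.
; Each change also swaps the button's red material, plays a plug sound and runs a timeline that lowers or raises the button.
; Overlaps are neither filtered nor counted, so any single exit releases the button.
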(event `self.TriggerBox.OnComponentBeginOverlap`
  (params (OverlappedComponent :type "PrimitiveComponent Object Reference") (OtherActor :type "Actor Object Reference") (OtherComp :type "PrimitiveComponent Object Reference") (OtherBodyIndex :type Integer) (bFromSweep :type Boolean) (SweepResult :type "HitResult Structure (by ref)"))
  (message `/Game/Blueprints/InteractableObject.InteractedEvent` (`self.Object`))
  (message `/Game/Blueprints/InteractableObject.InteractedEvent` (`self.Object2`))
  (`PrimitiveComponent.SetMaterial` (`self.button`) 0 "/Game/Material/Red_off.Red_off")
  (`GameplayStatics.PlaySoundAtLocation` "/Game/Sounds/Misc_SFX/Electronics__Electrical_Socket_Safety_Cover__Plug_In_SND25693.Electronics__Electrical_Socket_Safety_Cover__Plug_In_SND25693" (`self.K2_GetActorLocation`) (struct) 1.0 1.0 0.0 null null null)
  (bind (_direction _newtrack_0) (`Timeline|Timeline_0` :!via `PlayFromStart` :!label _label)
    (:`Update`
      (`SceneComponent.K2_SetRelativeLocation` (`self.button`) (`KismetMathLibrary.MakeVector` 0.0 0.0 (`KismetMathLibrary.Lerp` 0.0 -10.0 _newtrack_0)) false false))))

(event `self.TriggerBox.OnComponentEndOverlap`
  (params (OverlappedComponent :type "PrimitiveComponent Object Reference") (OtherActor :type "Actor Object Reference") (OtherComp :type "PrimitiveComponent Object Reference") (OtherBodyIndex :type Integer))
  (message `/Game/Blueprints/InteractableObject.StopedInteractedEvent` (`self.Object`))
  (message `/Game/Blueprints/InteractableObject.StopedInteractedEvent` (`self.Object2`))
  (`PrimitiveComponent.SetMaterial` (`self.button`) 0 "/Game/Material/Red.Red")
  (`GameplayStatics.PlaySoundAtLocation` "/Game/Sounds/Misc_SFX/Electronics__Electrical_Socket_Safety_Cover__Plug_Remove_SND25692.Electronics__Electrical_Socket_Safety_Cover__Plug_Remove_SND25692" (`self.K2_GetActorLocation`) (struct) 1.0 1.0 0.0 null null null)
  (goto _label :!via `ReverseFromEnd`))

(fn `NewFunction_0`)

(fn `UserConstructionScript`)