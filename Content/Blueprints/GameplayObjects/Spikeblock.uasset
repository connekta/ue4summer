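; Interactable spike block that moves its Spikes component vertically to a configurable height while interacted with.
; BeginPlay caches the starting relative location and derives the end point by replacing Z with SetHeight.
; A timeline plays on InteractedEvent and reverses on StopedInteractedEvent, lerping the spikes between both points.
; When SetHeight exceeds a threshold, the same timeline alpha also stretches the spikes along Z.
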(event `self.ReceiveBeginPlay`
  (bind _relativelocation (`SceneComponent.RelativeLocation` (`self.spikes`)))
  (set `self.StartPos` _relativelocation)
  (set `self.EndPos` (`KismetMathLibrary.MakeVector` (.x _relativelocation) (.y _relativelocation) (`self.SetHeight`))))

(event `/Game/Blueprints/InteractableObject.InteractedEvent`
  (bind _spikes (`self.spikes`))
  (bind (_direction _newtrack_0) (`Timeline|Timeline_0` :`NewTime` 0.0 :!label _label)
    (:`Update`
      (`|ExecutionSequence`
        (:`then_0`
          (`SceneComponent.K2_SetRelativeLocation` _spikes (`KismetMathLibrary.VLerp` (`self.StartPos`) (`self.EndPos`) _newtrack_0) false false))
        (:`then_1`
          (if (> (`self.SetHeight`) 150.0)
            (`SceneComponent.SetRelativeScale3D` _spikes (`KismetMathLibrary.VLerp` (1.0 1.0 1.0) (1.0 1.0 1.5) _newtrack_0))))))))

(event `/Game/Blueprints/InteractableObject.StopedInteractedEvent`
  (goto _label :!via `Reverse`))

(fn `UserConstructionScript`)