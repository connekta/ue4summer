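; Level goal trigger for local multiplayer that shows a win widget and loads NextLevel, or MenuMap if None, after five seconds.
; With WaitForAll, each begin overlap recounts GM_LocalMP's SpawnedActors, winning when all are dead or inside; otherwise any overlap wins.
; The text shows living players inside against HowManyPlayersNeeded, using a short Delay so the second Sequence branch counts the dead first.
; The count has no end-overlap update.
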(event `self.ReceiveBeginPlay`
  (if (`self.WaitForAll`)
    (`TextRenderComponent.K2_SetText` (`self.Number of PlayersInside`) (`KismetTextLibrary.Conv_StringToText` (`KismetStringLibrary.Concat_StrStr` (`KismetStringLibrary.Conv_IntToString` (`self.NumberOfOverlappingActors`)) "/" (`self.HowManyPlayersNeeded?`))))))

(event `self.WinTrigger.OnComponentBeginOverlap`
  (params (OverlappedComponent :type "PrimitiveComponent Object Reference") (OtherActor :type "Actor Object Reference") (OtherComp :type "PrimitiveComponent Object Reference") (OtherBodyIndex :type Integer) (bFromSweep :type Boolean) (SweepResult :type "HitResult Structure (by ref)"))
  (bind _nextlevel (`self.NextLevel`))
  (if (`self.WaitForAll`)
    (set `self.NumberOfOverlappingActors` 0)
    (set `self.numberofdeadchars` 0)
    (bind _asgm_local_mp (cast `/Game/Assets/Blueprints/GM_LocalMP` (`GameplayStatics.GetGameMode`)))
    (bind _spawnedactors (`/Game/Assets/Blueprints/GM_LocalMP.SpawnedActors` _asgm_local_mp))
    (set `self.TotalNumberOfActors` (`KismetArrayLibrary.Array_Length` _spawnedactors))
    (`|ExecutionSequence`
      (:`then_0`
        (for _array_element _spawnedactors
          (if (or (`/Game/Assets/Blueprints/BP_Player.is_dead` _array_element) (`PrimitiveComponent.IsOverlappingActor` (`self.WinTrigger`) _array_element))
            (`/Engine/EditorBlueprintResources/StandardMacros.IncrementInt` (`self.NumberOfOverlappingActors`))))
        (`KismetSystemLibrary.Delay` 0.2)
        (`TextRenderComponent.K2_SetText` (`self.Number of PlayersInside`) (`KismetTextLibrary.Conv_StringToText` (`KismetStringLibrary.Concat_StrStr` (`KismetStringLibrary.Conv_IntToString` (- (`self.NumberOfOverlappingActors`) (`self.numberofdeadchars`))) " / " (`self.HowManyPlayersNeeded?`))))
        (if (== (`self.NumberOfOverlappingActors`) (`self.TotalNumberOfActors`))
          ;[1 1 1] Show Win Widget And Load Next Level
          (bind _returnvalue (`|CreateWidget` "/Game/Levels/WinWidget.WinWidget_C" :!label _label))
          (`UserWidget.AddToViewport` _returnvalue 0)
          (set `/Game/Levels/WinWidget.NextLevel` _nextlevel _returnvalue)
          (`WidgetBlueprintLibrary.SetInputMode_UIOnlyEx` (`GameplayStatics.GetPlayerController` 0) _returnvalue)
          (`KismetSystemLibrary.Delay` 5.0)
          (bind _asgm_local_mp_2 (cast `/Game/Assets/Blueprints/GM_LocalMP` (`GameplayStatics.GetGameMode`)))
          (if (== _nextlevel "None")
            (`/Game/Assets/Blueprints/GM_LocalMP.LoadNextLevel` _asgm_local_mp_2 "MenuMap")
            (else
              (`/Game/Assets/Blueprints/GM_LocalMP.LoadNextLevel` _asgm_local_mp_2 _nextlevel)))))
      (:`then_1`
        (for _array_element_2 _spawnedactors
          (if (`/Game/Assets/Blueprints/BP_Player.is_dead` _array_element_2)
            (`/Engine/EditorBlueprintResources/StandardMacros.IncrementInt` (`self.numberofdeadchars`))))))
    (else
      (goto _label))))

(fn `UserConstructionScript`)