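; Moving platform gameplay object that slides along its local Y axis, with two cogs that turn in step with the motion.
; A timeline starts on BeginPlay, and its track scaled by Distance sets the Y position of the Billboard component without sweeping.
; The same track drives the roll of both cogs across two full turns, keeping their spin locked to the travel.
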(event `self.ReceiveBeginPlay`
  (bind _billboard (`self.Billboard`))
  (bind (_direction _newtrack_0) (`Timeline|Timeline_0`)
    (:`Update`
      (`SceneComponent.K2_SetRelativeLocation` _billboard (`KismetMathLibrary.MakeVector` (.x (`SceneComponent.RelativeLocation` _billboard)) (* _newtrack_0 (`self.Distance`)) (.z (`SceneComponent.RelativeLocation` _billboard))) false false)
      (`SceneComponent.K2_SetRelativeRotation` (`self.cogs1`) (`KismetMathLibrary.MakeRotator` (`KismetMathLibrary.Lerp` 0.0 720.0 _newtrack_0)) false false)
      (`SceneComponent.K2_SetRelativeRotation` (`self.cogs2`) (`KismetMathLibrary.MakeRotator` (`KismetMathLibrary.Lerp` 0.0 720.0 _newtrack_0)) false false))))

(fn `UserConstructionScript`)